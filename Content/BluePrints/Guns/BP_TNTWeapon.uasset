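; TNT revolver weapon Blueprint that shows a placeholder bullet on the gun while no shot is in progress.
; BeginPlay sets the TNT revolver skeletal mesh on Weapon and snaps BulletTemp to its Bullet_Socket, an attachment the construction script also makes.
; Each Tick casts the Weapon component's owner to PlayerCharacter and, if that succeeds, hides BulletTemp in game whenever IsShooting is true.
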(event EventBeginPlay
  (Class|SkinnedMeshComponent|SetSkeletalMesh (Variables|Default|GetWeapon) "/Game/Assets/Weapons/Non-Melee_Weapons/TntRevolver/TntRevolver_SKM.TntRevolver_SKM" true)
  (Transformation|AttachComponentToComponent (Variables|Default|GetBullet_Temp) (Variables|Default|GetWeapon) "Bullet_Socket" "SnapToTarget" "KeepWorld" "SnapToTarget" true))

(event Collision|EventActorBeginOverlap
  (params (OtherActor :type Actor%20Object%20Reference)))

(event EventTick
  (params (DeltaSeconds :type Float%20%28single-precision%29))
  (bind _asplayer_character (Utilities|Casting|CastToPlayerCharacter (Components|GetOwner (Variables|Default|GetWeapon))))
  (Development|SetHiddeninGame (Variables|Default|GetBullet_Temp) (Variables|/Script/TerrorTrains.PlayerCharacter|GetIsShooting _asplayer_character) false))

(fn ConstructionScript
  (Transformation|AttachComponentToComponent (Variables|Default|GetBullet_Temp) (Variables|Default|GetWeapon) "Bullet_Socket" "SnapToTarget" "KeepRelative" "KeepRelative" true))