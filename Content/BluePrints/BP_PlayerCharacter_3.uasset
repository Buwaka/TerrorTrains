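; Cowboy player character Blueprint that wears a hat and poncho and displays health and player-number widgets.
; BeginPlay caches max health, socket-attaches both accessories and passes the player index to Cowboy_AnimBP after a short delay working around wrong early indexes.
; Tick pushes the health fraction to the HealthWidget and rotates the indicator toward camera manager 1.
; DoOnce gates label the indicator with number and color, then hide it after its lifetime.
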(event EventBeginPlay
  (bind _mesh (Variables|Character|GetMesh))
  (Utilities|FlowControl|Sequence
    (:then_0
      (bind _returnvalue (Class|HealthComponent|GetHealth (Variables|Default|GetHealth)))
      (Variables|Default|SetMaxHealth _returnvalue)
      (Utilities|FlowControl|Delay 0.2) ; 1St frame indexes appear to be wring
      (bind _ascowboy_anim_bp (Utilities|Casting|CastToCowboy_AnimBP (Components|SkeletalMesh|GetAnimInstance (Variables|Character|GetMesh))))
      (bind _output_get (Variables|/Game/Assets/Characters/Main_Characters/Cowboy_AnimBP.Cowboy_AnimBP_C|SetplayerIndex _ascowboy_anim_bp (Class|PlayerCharacter|GetPlayerIndex self))))
    (:then_1
      (Transformation|AttachComponentToComponent (Variables|Default|GetHat_Bandana_SM) _mesh "Hat_Socket" "SnapToTarget" "SnapToTarget" "KeepRelative" true))
    (:then_2
      (Transformation|AttachComponentToComponent (Variables|Default|GetPoncho_Default_SM) _mesh "Poncho_Socket" "SnapToTarget" "SnapToTarget" "KeepRelative" true))))

(event EventTick
  (params (DeltaSeconds :type Float%20%28single-precision%29))
  (bind _ashealth_widget (Utilities|Casting|CastToHealthWidget (UserInterface|GetUserWidgetObject (Variables|Default|GetWidget))))
  (bind _returnvalue (Class|HealthComponent|GetHealth (Variables|Default|GetHealth)))
  (Default|SetHealth _ashealth_widget (/ _returnvalue (Variables|Default|GetMaxHealth)))
  (CallFunction|HandlePlayerIndicator)
  (if (>= (Actor|GetGameTimeSinceCreation) (Variables|Default|GetPlayerIndicatorLifeTime))
    (Utilities|FlowControl|DoOnce false
      (:Completed
        (Variables|Default|SetShowIndicator false)))
    (else
      (Utilities|FlowControl|DoOnce false
        (:Completed
          (CallFunction|SetPlayerIndicator))))))

(fn ConstructionScript)

(fn HandlePlayerIndicator
  (bind _showindicator (Variables|Default|GetShowIndicator))
  (bind _indicatorscale (Variables|Default|GetIndicatorScale))
  (Transformation|SetWorldRotation (Variables|Default|GetIndicator) (Math|Rotator|FindLookatRotation (Transformation|GetWorldLocation (Variables|Default|GetCapsuleComponent)) (Camera|GetCameraLocation (Game|GetPlayerCameraManager 1))) false false)
  (Rendering|SetVisibility (Variables|Default|GetIndicator) _showindicator false)
  (if _showindicator
    (Transformation|SetRelativeScale3D (Variables|Default|GetIndicator) (Math|Vector|MakeVector _indicatorscale _indicatorscale _indicatorscale))))

(fn SetPlayerIndicator
  (bind _asplayer_indicator (Utilities|Casting|CastToPlayerIndicator (UserInterface|GetUserWidgetObject (Variables|Default|GetIndicator))))
  (Default|UpdatePlayer _asplayer_indicator (+ (Class|PlayerCharacter|GetPlayerIndex) 1) (Variables|Default|GetIndicatorColor)))