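; Locomotive2 is a train locomotive Blueprint that drives its smoke and brake spark effects from the train's movement state.
; Each Tick polls GetIsStopped to pause and reset the smoke while stopped, or unpause it while moving.
; It also polls GetIsBreaking to unpause four spark systems while braking, and otherwise pauses and resets them every frame.
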(event EventTick
  (params (DeltaSeconds :type Float%20%28single-precision%29))
  (bind _break_sparks4 (Variables|Default|GetBreak_Sparks4))
  (bind _break_sparks1 (Variables|Default|GetBreak_Sparks1))
  (bind _break_sparks2 (Variables|Default|GetBreak_Sparks2))
  (bind _break_sparks3 (Variables|Default|GetBreak_Sparks3))
  (bind _locomotive_smoke (Variables|Default|GetLocomotive_Smoke))
  (bind _returnvalue (Class|Train|GetIsStopped))
  (if _returnvalue
    ;[1 0.25 0.25] Train is not moving
    (Class|NiagaraComponent|SetPaused _locomotive_smoke true)
    (Niagara|ResetSystem _locomotive_smoke)
    (else
      ;[0.4973 1 0.531] Train is moving
      (Class|NiagaraComponent|SetPaused (Variables|Default|GetLocomotive_Smoke) false)))
  (bind _returnvalue_2 (Class|Train|GetIsBreaking))
  (if _returnvalue_2
    ;[1 0.1927 0.1927] Train is Breaking
    (Utilities|FlowControl|Sequence
      (:then_0
        (Class|NiagaraComponent|SetPaused (Variables|Default|GetBreak_Sparks1) false))
      (:then_1
        (Class|NiagaraComponent|SetPaused (Variables|Default|GetBreak_Sparks2) false))
      (:then_2
        (Class|NiagaraComponent|SetPaused (Variables|Default|GetBreak_Sparks3) false))
      (:then_3
        (Class|NiagaraComponent|SetPaused (Variables|Default|GetBreak_Sparks4) false)))
    (else
      ;[0.4271 1 0.4927] Train is not Breaking
      (Utilities|FlowControl|Sequence
        (:then_0
          (Class|NiagaraComponent|SetPaused _break_sparks1 true)
          (Niagara|ResetSystem _break_sparks1))
        (:then_1
          (Class|NiagaraComponent|SetPaused _break_sparks2 true)
          (Niagara|ResetSystem _break_sparks2))
        (:then_2
          (Class|NiagaraComponent|SetPaused _break_sparks3 true)
          (Niagara|ResetSystem _break_sparks3))
        (:then_3
          (Class|NiagaraComponent|SetPaused _break_sparks4 true)
          (Niagara|ResetSystem _break_sparks4))))))

(fn ConstructionScript)