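; Blue storage wagon Blueprint for a train, with four brake spark effect components.
; Two sequences in the event graph are meant to toggle the sparks by swapping each component's asset between a sparks system and an empty one for braking and non-braking states.
; Neither sequence is connected to an event, so the toggle never runs, and the construction script is empty.
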(fn ConstructionScript)