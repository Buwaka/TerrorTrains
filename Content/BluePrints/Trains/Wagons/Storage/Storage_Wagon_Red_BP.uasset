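; Red storage wagon Blueprint for a train, with four Niagara components for braking sparks.
; Two Event Graph fragments swap all four components between a sparks system and an empty system for the braking and non-braking states.
; Neither fragment is connected to an event, so the switch never runs, and the construction script is empty.
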(fn ConstructionScript)