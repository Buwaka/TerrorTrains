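; BP_Latern is a decorative train-wagon lantern with a configurable rect light and an optional swing.
; The construction script applies light color, intensity, attenuation radius and square source size, and disables collision on the static mesh.
; When Swing is set, BeginPlay starts a looping timer at a configurable update rate in place of Tick.
; Each update sets the Arrow's world rotation from a nested sine of offset game time, shaped by a FallOff exponent.
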(event Custom|Update
  (Transformation|SetWorldRotation (Variables|Default|GetArrow) (* (Variables|Default|Swing|GetSwing_Angle) (Math|Trig|Sin(Degrees) (Math|Float|Power (* (Math|Trig|Sin(Degrees) (* (+ (Utilities|Time|GetGameTimeinSeconds) (Variables|Default|Swing|GetStartingOffset)) (Variables|Default|Swing|GetSpeed))) (Variables|Default|Swing|GetSpeed)) (Variables|Default|Swing|GetFallOff)))) false false))

(event EventBeginPlay
  (if (Variables|Default|GetSwing?)
    (Utilities|Time|SetTimerbyEvent (delegate Custom|Update) (* (/ 6e+01 (Variables|Default|GetUpdateRate%28FPS%29)) 0.016) true)))

(event Collision|EventActorBeginOverlap
  (params (OtherActor :type Actor%20Object%20Reference)))

(event EventTick
  (params (DeltaSeconds :type Float%20%28single-precision%29)))

(fn ConstructionScript
  (bind _rectlight (Variables|Default|GetRectLight))
  (bind _size (Variables|Default|Light|GetSize))
  (Rendering|Components|Light|SetLightColor _rectlight (Variables|Default|Light|GetLight%20Color) true)
  (Rendering|Components|Light|SetIntensity _rectlight (Variables|Default|Light|GetLight%20Intensity))
  ;[1 1 1] ATT Rad
  (Rendering|Lighting|SetAttenuationRadius _rectlight (Variables|Default|Light|GetAtt%20Radius))
  ;[1 1 1] Size
  (Class|RectLightComponent|SetSourceWidth _rectlight _size)
  (Class|RectLightComponent|SetSourceHeight _rectlight _size)
  ;[1 1 1] Collision
  (Collision|SetCollisionEnabled (Variables|Default|GetStaticMesh) "NoCollision"))