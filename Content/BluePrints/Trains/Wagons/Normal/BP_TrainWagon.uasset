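; Train wagon Blueprint that drives Niagara effects for station stops and braking, based on the state of its owning Train.
; Each Tick, the wagon's team selects a pair of exit emitters and the Down or Up exit system.
; A DoOnce restarts that effect with a station time when the train stops, then re-arms and swaps in an empty system while moving.
; Four brake spark systems unpause while braking, otherwise pause and reset.
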(event EventTick
  (params (DeltaSeconds :type Float%20%28single-precision%29))
  (bind _train_exit (Variables|Default|GetTrain_Exit))
  (bind _break_sparks4 (Variables|Default|GetBreak_Sparks4))
  (bind _break_sparks1 (Variables|Default|GetBreak_Sparks1))
  (bind _break_sparks2 (Variables|Default|GetBreak_Sparks2))
  (bind _break_sparks3 (Variables|Default|GetBreak_Sparks3))
  (bind _train_exit2 (Variables|Default|GetTrain_Exit2))
  (bind _niagara (Variables|Default|GetNiagara))
  (bind _niagara1 (Variables|Default|GetNiagara1))
  (bind _astrain (Utilities|Casting|CastToTrain (Components|GetOwner)))
  (bind _returnvalue (Class|TrainWagon|GetTeam))
  (if (== _returnvalue 1)
    (bind _returnvalue_2 (Class|Train|GetIsStopped _astrain))
    ;[1 0.8247 0.4678] Train comes to a stop
    (if _returnvalue_2
      (Utilities|FlowControl|Sequence
        (:then_0
          (Utilities|FlowControl|DoOnce true :!label _label
            (:Completed
              (Class|NiagaraComponent|SetAsset (Variables|Default|GetTrain_Exit) "/Game/Assets/Particles/Train_Exit/Train_Exit_Down_NS.Train_Exit_Down_NS")
              (Class|NiagaraComponent|SetAsset (Variables|Default|GetTrain_Exit2) "/Game/Assets/Particles/Train_Exit/Train_Exit_Down_NS.Train_Exit_Down_NS")
              (Variables|Default|SetStationTime 4e+01)
              (Niagara|SetNiagaraVariable(Float) _train_exit "User.StationTime" (Variables|Default|GetStationTime))
              (Niagara|SetNiagaraVariable(Float) _train_exit2 "User.StationTime" (Variables|Default|GetStationTime))
              (Niagara|ResetSystem _train_exit)
              (Niagara|ResetSystem _train_exit2))))
        (:then_1
          (bind _returnvalue_3 (Class|Train|GetIsBreaking _astrain :!label _label_2))
          (if _returnvalue_3
            ;[1 0.1927 0.1927] Train is Breaking
            (Utilities|FlowControl|Sequence :!label _label_3
              (:then_0
                (Class|NiagaraComponent|SetPaused (Variables|Default|GetBreak_Sparks1) false))
              (:then_1
                (Class|NiagaraComponent|SetPaused (Variables|Default|GetBreak_Sparks2) false))
              (:then_2
                (Class|NiagaraComponent|SetPaused (Variables|Default|GetBreak_Sparks3) false))
              (:then_3
                (Class|NiagaraComponent|SetPaused (Variables|Default|GetBreak_Sparks4) false)))
            (else
              ;[0.4271 1 0.4927] Train is not Breaking
              (Utilities|FlowControl|Sequence :!label _label_4
                (:then_0
                  (Class|NiagaraComponent|SetPaused _break_sparks1 true)
                  (Niagara|ResetSystem _break_sparks1))
                (:then_1
                  (Class|NiagaraComponent|SetPaused _break_sparks2 true)
                  (Niagara|ResetSystem _break_sparks2))
                (:then_2
                  (Class|NiagaraComponent|SetPaused _break_sparks3 true)
                  (Niagara|ResetSystem _break_sparks3))
                (:then_3
                  (Class|NiagaraComponent|SetPaused _break_sparks4 true)
                  (Niagara|ResetSystem _break_sparks4)))))))
      (else
        (Class|NiagaraComponent|SetAsset (Variables|Default|GetTrain_Exit) "/Game/Assets/Particles/Break_Sparks/Break_Empty_NS.Break_Empty_NS")
        (Class|NiagaraComponent|SetAsset (Variables|Default|GetTrain_Exit2) "/Game/Assets/Particles/Break_Sparks/Break_Empty_NS.Break_Empty_NS")
        (Utilities|FlowControl|Sequence
          (:then_0
            (goto _label Reset))
          (:then_1
            (goto _label_2)))))
    (else
      (bind _returnvalue_4 (Class|Train|GetIsStopped _astrain))
      ;[1 0.8247 0.4678] Train comes to a stop
      (if _returnvalue_4
        (Utilities|FlowControl|Sequence
          (:then_0
            (Utilities|FlowControl|DoOnce true :!label _label_5
              (:Completed
                (Class|NiagaraComponent|SetAsset (Variables|Default|GetNiagara) "/Game/Assets/Particles/Train_Exit/Train_Exit_Up_NS.Train_Exit_Up_NS")
                (Class|NiagaraComponent|SetAsset (Variables|Default|GetNiagara1) "/Game/Assets/Particles/Train_Exit/Train_Exit_Up_NS.Train_Exit_Up_NS")
                (Variables|Default|SetStationTime 4e+01)
                (Niagara|SetNiagaraVariable(Float) _niagara "User.StationTime" (Variables|Default|GetStationTime))
                (Niagara|SetNiagaraVariable(Float) _niagara1 "User.StationTime" (Variables|Default|GetStationTime))
                (Niagara|ResetSystem _niagara)
                (Niagara|ResetSystem _niagara1))))
          (:then_1
            (bind _returnvalue_5 (Class|Train|GetIsBreaking _astrain :!label _label_6))
            (if _returnvalue_5
              (goto _label_3)
              (else
                (goto _label_4)))))
        (else
          (Class|NiagaraComponent|SetAsset (Variables|Default|GetNiagara) "/Game/Assets/Particles/Break_Sparks/Break_Empty_NS.Break_Empty_NS")
          (Class|NiagaraComponent|SetAsset (Variables|Default|GetNiagara1) "/Game/Assets/Particles/Break_Sparks/Break_Empty_NS.Break_Empty_NS")
          (Utilities|FlowControl|Sequence
            (:then_0
              (goto _label_5 Reset))
            (:then_1
              (goto _label_6))))))))

(fn ConstructionScript)